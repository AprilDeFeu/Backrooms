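; BP_RB_Maze generates a seeded recursive-backtracker maze in the Construction Script, placing a Hierarchical Instanced Static Mesh instance on each path cell.
; CreateMaze starts at a random cell, and AddNeighbourPosition recursively carves to valid neighbours two cells away, trying directions from a random start.
; Backtrack pops pending cells and moves their connecting wall cells into the path.
; Dead ends are collected and returned, but the Construction Script ignores them.
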(event EventBeginPlay)

(event Collision|EventActorBeginOverlap
  (params (OtherActor :type Actor%20Object%20Reference)))

(event EventTick
  (params (DeltaSeconds :type Float%20%28single-precision%29)))

(fn ConstructionScript
  (bind _cellsize (Variables|Default|GetcellSize))
  (bind _outputpath (CallFunction|CreateMaze (Variables|Default|GetmazeSize) (Variables|Default|GetmazeSeed)))
  (bind _result (Utilities|Set|ToArray _outputpath))
  (for _array_element _result
    (Components|InstancedStaticMesh|AddInstance (Variables|Default|GetHierarchicalInstancedStaticMesh) (Math|Transform|MakeTransform (Math|Vector|MakeVector (* (.X (Utilities|Struct|BreakIntPoint _array_element)) _cellsize) (* (.Y (Utilities|Struct|BreakIntPoint _array_element)) _cellsize) 0.0)))))

(fn AddNeighbourPosition
  (params (mazeSize :type Int%20Point%20Structure%20%28by%20ref%29) (randStream :type Random%20Stream%20Structure%20%28by%20ref%29) (currentPosition :type Int%20Point%20Structure%20%28by%20ref%29) (path :type Set%20of%20Int%20Point%20Structures) (walls :type Set%20of%20Int%20Point%20Structures) (toVerify :type Set%20of%20Int%20Point%20Structures) (deadEnds :type Set%20of%20Int%20Point%20Structures))
  (LocalVariables|SetneighbourIndex (Math|Random|RandomIntegerinRangefromStream 0 3 randStream))
  (if (Utilities|ValidPosition (.neighbour (Utilities|GetNeighbourandWall currentPosition (LocalVariables|GetneighbourIndex))) mazeSize path walls) :!label _label
    (Utilities|Set|Add path (.neighbour (Utilities|GetNeighbourandWall currentPosition (LocalVariables|GetneighbourIndex))))
    (Utilities|Set|Add walls (.wall (Utilities|GetNeighbourandWall currentPosition (LocalVariables|GetneighbourIndex))))
    (Utilities|Set|Add toVerify (.neighbour (Utilities|GetNeighbourandWall currentPosition (LocalVariables|GetneighbourIndex))))
    (CallFunction|AddNeighbourPosition mazeSize randStream (.neighbour (Utilities|GetNeighbourandWall currentPosition (LocalVariables|GetneighbourIndex))) path walls toVerify deadEnds)
    (else
      (Utilities|RepeatN 4
        (:terminate
          (LocalVariables|SetneighbourIndex (Math|Integer|SelectInt 0 (+ 1 (LocalVariables|GetneighbourIndex)) (>= (+ 1 (LocalVariables|GetneighbourIndex)) 4)))
          (goto _label))
        (:overN
          (bind _count (CallFunction|NeighbourCount currentPosition path))
          (if (== _count 1)
            (Utilities|Set|Add deadEnds currentPosition)))))))

(fn CreateMaze
  (params (mazeSize :type Int%20Point%20Structure) (mazeSeed :type Integer))
  (Math|Random|SetRandomStreamSeed (LocalVariables|GetrandStream) mazeSeed)
  (LocalVariables|SetlocalMazeSize mazeSize)
  (bind _output_get (LocalVariables|SetinitialPosition (Utilities|RandomPosition (LocalVariables|GetlocalMazeSize) (LocalVariables|GetrandStream))))
  (LocalVariables|SetcurrentPosition _output_get)
  (CallFunction|AddNeighbourPosition (LocalVariables|GetlocalMazeSize) (LocalVariables|GetrandStream) (LocalVariables|GetcurrentPosition) (LocalVariables|GetlocalPath) (LocalVariables|GetlocalWalls) (LocalVariables|GetlocalVerify) (LocalVariables|GetlocalDeadEnds) :!label _label)
  (if (> (Utilities|Set|Length (LocalVariables|GetlocalVerify)) 0)
    (CallFunction|Backtrack (LocalVariables|GetcurrentPosition) (LocalVariables|GetlocalVerify) (LocalVariables|GetlocalPath) (LocalVariables|GetlocalWalls))
    (goto _label)
    (else
      (return (LocalVariables|GetlocalPath) (LocalVariables|GetlocalDeadEnds)))))

(fn NeighbourCount
  (params (currentPosition :type Int%20Point%20Structure%20%28by%20ref%29) (path :type Set%20of%20Int%20Point%20Structures))
  (for _array_element (Utilities|NeighbourPosition currentPosition)
    (if (Utilities|Set|Contains path _array_element)
      (Math|Integer|IncrementInt (LocalVariables|Getcounter))))
  (return (LocalVariables|Getcounter)))

(fn Backtrack
  (params (currentCell :type Int%20Point%20Structure%20%28by%20ref%29) (toVerify :type Set%20of%20Int%20Point%20Structures) (path :type Set%20of%20Int%20Point%20Structures) (walls :type Set%20of%20Int%20Point%20Structures))
  (bind _result (Utilities|Set|ToArray toVerify))
  (|SetBy-RefVar currentCell (Utilities|Array|Get(acopy) _result (Utilities|Array|LastIndex _result)))
  (Utilities|Set|Remove toVerify (Utilities|Array|Get(acopy) _result (Utilities|Array|LastIndex _result)))
  (bind _result_2 (Utilities|Set|ToArray walls))
  (Utilities|Set|Add path (Utilities|Array|Get(acopy) _result_2 (Utilities|Array|LastIndex _result_2)))
  (Utilities|Set|Remove walls (Utilities|Array|Get(acopy) _result_2 (Utilities|Array|LastIndex _result_2))))